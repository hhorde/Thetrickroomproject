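; Endless runner game mode that creates the HUD and lays the initial track at BeginPlay.
; AddFloorTile chains random straight tiles via each tile's attach transform, inserting jump pieces early in a straight run and a curve after a long run.
; Looping timers drive time and distance functions on MASTER_Values if play has begun at BeginPlay.
; Swipe events start looping timers for that actor's swipe display functions.
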(event Custom|Swipe%20Right%20to%20dodge
  (bind _returnvalue (Actor|GetActorOfClass "/Game/ThirdPersonBP/Blueprints/MASTER_Values.MASTER_Values_C"))
  (Utilities|Time|SetTimerbyFunctionName _returnvalue "DisplayPlayerSwiRight_FUNC" 2.0 true))

(event Custom|Swipe%20up%20tp%20jump
  (bind _returnvalue (Actor|GetActorOfClass "/Game/ThirdPersonBP/Blueprints/MASTER_Values.MASTER_Values_C"))
  (Utilities|Time|SetTimerbyFunctionName _returnvalue "DisplayPlayerSwipeup_FUNC" 2.0 true))

(event Custom|Swipe%20down%20to%20duck
  (bind _returnvalue (Actor|GetActorOfClass "/Game/ThirdPersonBP/Blueprints/MASTER_Values.MASTER_Values_C"))
  (Utilities|Time|SetTimerbyFunctionName _returnvalue "DisplayPlayerSwipeDown_FUNC" 2.0 true))

(event Custom|Swipe%20left%20to%20dodge
  (bind _returnvalue (Actor|GetActorOfClass "/Game/ThirdPersonBP/Blueprints/MASTER_Values.MASTER_Values_C"))
  (Utilities|Time|SetTimerbyFunctionName _returnvalue "DisplayPlayerSwipeLeft_FUNC" 2.0 true))

(event EventBeginPlay
  (bind _returnvalue (UserInterface|CreateWidget "/Game/ThirdPersonBP/Blueprints/HUD_Runnergame.HUD_Runnergame_C"))
  (UserInterface|Viewport|AddtoViewport _returnvalue 0)
  ;[1 1 1] check if game has begun after intro
  (Utilities|FlowControl|Sequence
    (:then_0
      ;[1 1 1] Plays function every second
      (bind _returnvalue_2 (Actor|GetActorOfClass "/Game/ThirdPersonBP/Blueprints/MASTER_Values.MASTER_Values_C"))
      (if (Variables|/Game/ThirdPersonBP/Blueprints/MASTER_Values.MASTER_Values_C|GetPlayerBeginsPlay_Bool _returnvalue_2)
        (Utilities|Time|SetTimerbyFunctionName _returnvalue_2 "AddOneToTime_FUNC" 1.0 true)
        (Utilities|Time|SetTimerbyFunctionName _returnvalue_2 "AddDistanceTraveled_FUNC" 0.6 true)
        (Utilities|Time|SetTimerbyFunctionName 0 "AddDistanceTraveled_FUNC" 2.0 true)))
    (:then_1
      (for _index (range 0 10)
        (CallFunction|AddFloorTile)))))

(event EventTick
  (params (DeltaSeconds :type Float%20%28single-precision%29)))

(event Input|KeyboardEvents|F
  (params (Key :type Key%20Structure))
  (:Pressed
    (Development|PrintString "Hello")))

(fn ConstructionScript)

(fn AddFloorTile
  (bind _floortiles (Variables|Default|GetFloorTiles))
  (if (> (Variables|Default|GetCurrentStraights) 7)
    (CallFunction|AddFloorCurve)
    (elif (Math|Integer|InRange(Integer) (Variables|Default|GetCurrentStraights) 1 3)
      (CallFunction|AddFloorJump)))
  (bind _returnvalue (Game|SpawnActorfromClass (Utilities|Array|Get(acopy) _floortiles (Math|Random|RandomIntegerinRange 0 (Utilities|Array|LastIndex _floortiles))) (Variables|Default|GetNextSpawnPoint) "Undefined" 0 0))
  (bind _asfloortile (Utilities|Casting|CastToFloortile _returnvalue))
  (bind _attachtransform (Default|GetAttachTransform _asfloortile))
  (Variables|Default|SetNextSpawnPoint _attachtransform)
  (Variables|Default|SetCurrentStraights (+ (Variables|Default|GetCurrentStraights) 1)))

(fn AddFloorCurve
  (bind _floorcurves (Variables|Default|GetFloorCurves))
  (bind _returnvalue (Game|SpawnActorfromClass (Utilities|Array|Get(acopy) _floorcurves (Math|Random|RandomIntegerinRange 0 (Utilities|Array|LastIndex _floorcurves))) (Variables|Default|GetNextSpawnPoint) "Undefined" 0 0))
  (bind _asfloortile (Utilities|Casting|CastToFloortile _returnvalue))
  (bind _attachtransform (Default|GetAttachTransform _asfloortile))
  (Variables|Default|SetNextSpawnPoint _attachtransform)
  (Variables|Default|SetCurrentStraights 0))

(fn AddFloorJump
  (bind _floorjumps (Variables|Default|GetFloorJumps))
  (bind _returnvalue (Game|SpawnActorfromClass (Utilities|Array|Get(acopy) _floorjumps (Math|Random|RandomIntegerinRange 0 (Utilities|Array|LastIndex _floorjumps))) (Variables|Default|GetNextSpawnPoint) "Undefined" 0 0))
  (bind _asfloortile (Utilities|Casting|CastToFloortile _returnvalue))
  (bind _attachtransform (Default|GetAttachTransform _asfloortile))
  (Variables|Default|SetNextSpawnPoint _attachtransform))